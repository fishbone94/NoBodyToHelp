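; BP_LaLlorona is an enemy that wanders, chases the player and sends them to the defeat menu on contact.
; Tick issues random navigable AI moves while it is neither moving nor in range.
; PawnSensing spotting the player raises walk speed and starts a chase, with a timer that later restores slow speed and clears the chase flag.
; Overlapping InteractSphere with the player opens the DefeatMenu level.
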(event OnComponentBeginOverlap(InteractSphere)
  (params (OverlappedComponent :type Primitive%20Component%20Object%20Reference) (OtherActor :type Actor%20Object%20Reference) (OtherComp :type Primitive%20Component%20Object%20Reference) (OtherBodyIndex :type Integer) (bFromSweep :type Boolean) (SweepResult :type Hit%20Result%20Structure%20%28by%20ref%29))
  (if (== (Utilities|GetClass OtherActor) "/Game/Core/BP_PlayerCharacter.BP_PlayerCharacter_C")
    (Game|OpenLevel(byName) "DefeatMenu")))

(event OnSeePawn(PawnSensing)
  (params (Pawn :type Pawn%20Object%20Reference))
  (if (== (Utilities|GetClass Pawn) "/Game/Core/BP_PlayerCharacter.BP_PlayerCharacter_C")
    (Variables|Default|SetInRange true)
    (Variables|/Script/Engine.CharacterMovementComponent|SetMaxWalkSpeed (Variables|Character|GetCharacterMovement) 4e+02)
    (AI|AIMoveTo self "0, 0, 0" Pawn 5.0 false
      (:then
        (bind _returnvalue (Utilities|Time|SetTimerbyEvent (delegate Custom|SlowDown) 2.0))))))

(event Custom|SlowDown
  (Variables|Default|SetInRange false)
  (Variables|/Script/Engine.CharacterMovementComponent|SetMaxWalkSpeed (Variables|Character|GetCharacterMovement) 1e+02)
  (Utilities|Time|ClearandInvalidateTimerbyHandle (stale OnSeePawn(PawnSensing) _returnvalue)))

(event EventBeginPlay)

(event Collision|EventActorBeginOverlap
  (params (OtherActor :type Actor%20Object%20Reference)))

(event EventTick
  (params (DeltaSeconds :type Float%20%28single-precision%29))
  (if (not (Variables|Default|GetIsMoving))
    (if (not (Variables|Default|GetInRange))
      (AI|AIMoveTo self (.RandomLocation (Class|NavigationSystem|GetRandomPointinNavigableRadius (Transformation|GetActorLocation) 1e+03)) 0 5.0 false
        (:then
          (Variables|Default|SetIsMoving true))
        (:OnSuccess
          (Variables|Default|SetIsMoving false :!label _label))
        (:OnFail
          (goto _label))))))

(fn ConstructionScript)