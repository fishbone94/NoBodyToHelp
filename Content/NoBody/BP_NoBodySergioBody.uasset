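; BP_NoBodySergioBody is a pawn that wanders the level autonomously.
; On Tick, while not already moving, it picks a random navigable point within a radius of its current location and sends itself there with AI MoveTo.
; An IsMoving flag blocks new requests during a move and clears on success or failure, so wandering repeats.
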(event EventBeginPlay
  (|CallParentFunction) ; This node is disabled and will not be called.\nDrag off pins to build functionality.
)

(event Collision|EventActorBeginOverlap
  (params (OtherActor :type Actor%20Object%20Reference))
  (|CallParentFunction OtherActor) ; This node is disabled and will not be called.\nDrag off pins to build functionality.
)

(event EventTick
  (params (DeltaSeconds :type Float%20%28single-precision%29))
  (|CallParentFunction DeltaSeconds)
  (if (not (Variables|Default|GetIsMoving))
    (AI|AIMoveTo self (.RandomLocation (Class|NavigationSystem|GetRandomPointinNavigableRadius (Transformation|GetActorLocation) 1e+03)) 0 5.0 false
      (:then
        (Variables|Default|SetIsMoving true))
      (:OnSuccess
        (Variables|Default|SetIsMoving false :!label _label))
      (:OnFail
        (goto _label)))))

(fn ConstructionScript
  (|CallParentFunction))